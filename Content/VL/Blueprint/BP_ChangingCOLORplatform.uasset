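; A platform Blueprint that starts pink and, when its Blue flag is set, briefly turns blue after the first-person character overlaps it.
; The Collision overlap starts a chain of delays that fires attached force feedback and prints "JUMP!" just before swapping the emissive material to blue.
; A Resetting event restores pink afterwards; without the flag, the overlap only triggers that delayed reset.
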(event `self.ReceiveBeginPlay`
  ;[0.3089 0.3854 1 0.5] Changing Color
  (`PrimitiveComponent.SetMaterial` (`self.Platform`) 0 "/Game/VL/Material/NeonLights/PlatformEmissives/M_Emissive_Pink.M_Emissive_Pink") ; Pink
)

(event `Resetting`
  ;[0.3089 0.3854 1 0.5] Changing Color
  (`PrimitiveComponent.SetMaterial` (`self.Platform`) 0 "/Game/VL/Material/NeonLights/PlatformEmissives/M_Emissive_Pink.M_Emissive_Pink") ; Pink
)

(event `self.Collision.OnComponentBeginOverlap`
  (params (OverlappedComponent :type "PrimitiveComponent Object Reference") (OtherActor :type "Actor Object Reference") (OtherComp :type "PrimitiveComponent Object Reference") (OtherBodyIndex :type Integer) (bFromSweep :type Boolean) (SweepResult :type "HitResult Structure (by ref)"))
  ;[0.3089 0.3854 1 0.5] Changing Color
  ;;[0.7777 0.3259 0.8906 0.5] Player Interaction
  (cast `/Game/FirstPerson/Blueprints/BP_FirstPersonCharacter` OtherActor)
  (if (`self.bBlue?`)
    (`KismetSystemLibrary.Delay` 0.35)
    (`GameplayStatics.SpawnForceFeedbackAttached` "/Game/ForceFeedback/FFE_ColorChaning.FFE_ColorChaning" (`self.Collision`) "None" (0.0 0.0 0.0) (struct) "KeepRelativeOffset" false false 1.0 0.0 null)
    (`KismetSystemLibrary.PrintString` "JUMP!" true true (struct :`R` 1.0 :`B` 0.562782 :`A` 1.0))
    (`KismetSystemLibrary.Delay` 0.15)
    (`PrimitiveComponent.SetMaterial` (`self.Platform`) 0 "/Game/VL/Material/NeonLights/PlatformEmissives/M_Emissive_Blue.M_Emissive_Blue") ; Blue
    (`KismetSystemLibrary.Delay` 0.5)
    (`self.Resetting`)
    (else
      (`KismetSystemLibrary.Delay` 0.5)
      (`self.Resetting`))))

(fn `UserConstructionScript`)