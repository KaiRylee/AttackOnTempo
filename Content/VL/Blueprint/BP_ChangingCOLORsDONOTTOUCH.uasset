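; Hazard platform that cycles its emissive color and triggers game over when the first-person character enters its kill zone.
; BeginPlay creates the game-over widget, then swaps the platform material through four colors on half-second delays, re-entering the sequence via a for loop.
; The Killzone overlap ignores the current color: it prints a warning, shows the widget, pauses the game and switches to UI-only input with a cursor.
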(event `self.ReceiveBeginPlay`
  ;[0.3089 0.3854 1 0.5] Changing Color
  (bind _returnvalue (`|CreateWidget` "/Game/Emma/UI/W_GameOVer.W_GameOVer_C"))
  (set `self.Game Over Widget` _returnvalue)
  (`PrimitiveComponent.SetMaterial` (`self.Platform`) 0 "/Game/VL/Material/NeonLights/PlatformEmissives/M_Emissive_Purple.M_Emissive_Purple" :!label _label) ; Pink
  (`KismetSystemLibrary.Delay` 0.5)
  (`PrimitiveComponent.SetMaterial` (`self.Platform`) 0 "/Game/VL/Material/NeonLights/PlatformEmissives/M_Emissive_Yellow.M_Emissive_Yellow") ; Blue
  (`KismetSystemLibrary.Delay` 0.5)
  (`PrimitiveComponent.SetMaterial` (`self.Platform`) 0 "/Game/VL/Material/NeonLights/PlatformEmissives/MI_Emissive_Green.MI_Emissive_Green") ; Blue
  (`KismetSystemLibrary.Delay` 0.5)
  (`PrimitiveComponent.SetMaterial` (`self.Platform`) 0 "/Game/VL/Material/NeonLights/PlatformEmissives/M_Emissive_Red.M_Emissive_Red") ; Blue
  (`KismetSystemLibrary.Delay` 0.5)
  (for _ (range 21)
    (goto _label)))

(event `self.Killzone.OnComponentBeginOverlap`
  (params (OverlappedComponent :type "PrimitiveComponent Object Reference") (OtherActor :type "Actor Object Reference") (OtherComp :type "PrimitiveComponent Object Reference") (OtherBodyIndex :type Integer) (bFromSweep :type Boolean) (SweepResult :type "HitResult Structure (by ref)"))
  (bind _returnvalue (`GameplayStatics.GetPlayerController` 0))
  ;[0.3089 0.3854 1 0.5] Changing Color
  ;;[0.7777 0.3259 0.8906 0.5] kill player
  (cast `/Game/FirstPerson/Blueprints/BP_FirstPersonCharacter` OtherActor)
  (`KismetSystemLibrary.PrintString` "WRONG COLOR!")
  (`UserWidget.AddToViewport` (`self.Game Over Widget`) 0)
  (`GameplayStatics.SetGamePaused` true)
  (`WidgetBlueprintLibrary.SetInputMode_UIOnlyEx` _returnvalue null)
  (set `PlayerController.bShowMouseCursor` true _returnvalue))

(fn `UserConstructionScript`)