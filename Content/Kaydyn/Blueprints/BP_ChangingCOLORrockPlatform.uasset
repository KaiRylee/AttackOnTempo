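; Rock platform actor that flashes between pink and blue and signals the player to jump when stepped on.
; BeginPlay alternates emissive materials on half-second delays, with a ForLoop wired back to the start so the cycle keeps repeating.
; When BP_FirstPersonCharacter overlaps Collision, a short delay precedes force feedback, a "JUMP!" debug print and a legacy camera shake.
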(event `self.ReceiveBeginPlay`
  ;[0.3089 0.3854 1 0.5] Changing Color
  ;;[0.7777 0.3259 0.8906 0.5] Player Interaction
  (`PrimitiveComponent.SetMaterial` (`self.Platform`) 0 "/Game/VL/Material/NeonLights/PlatformEmissives/M_Emissive_Pink.M_Emissive_Pink" :!label _label) ; Pink
  (`KismetSystemLibrary.Delay` 0.5)
  (`PrimitiveComponent.SetMaterial` (`self.Platform`) 0 "/Game/VL/Material/NeonLights/PlatformEmissives/M_Emissive_Blue.M_Emissive_Blue") ; Blue
  (`KismetSystemLibrary.Delay` 0.5)
  (for _ (range 21)
    (goto _label)))

(event `self.Collision.OnComponentBeginOverlap`
  (params (OverlappedComponent :type "PrimitiveComponent Object Reference") (OtherActor :type "Actor Object Reference") (OtherComp :type "PrimitiveComponent Object Reference") (OtherBodyIndex :type Integer) (bFromSweep :type Boolean) (SweepResult :type "HitResult Structure (by ref)"))
  ;[0.3089 0.3854 1 0.5] Changing Color
  ;;[0.7777 0.3259 0.8906 0.5] Player Interaction
  (cast `/Game/FirstPerson/Blueprints/BP_FirstPersonCharacter` OtherActor)
  (`KismetSystemLibrary.Delay` 0.35)
  (`GameplayStatics.SpawnForceFeedbackAttached` "/Game/ForceFeedback/FFE_ColorChaning.FFE_ColorChaning" (`self.Collision`) "None" (0.0 0.0 0.0) (struct) "KeepRelativeOffset" false false 1.0 0.0 null)
  (`KismetSystemLibrary.PrintString` "JUMP!" true true (struct :`R` 1.0 :`B` 0.562782 :`A` 1.0))
  (`LegacyCameraShake.StartLegacyCameraShake` (`GameplayStatics.GetPlayerCameraManager` 0) "/Game/CameraShake/LCS_Platform.LCS_Platform_C"))

(fn `UserConstructionScript`)